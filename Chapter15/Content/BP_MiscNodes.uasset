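; BP_MiscNodes is a Blueprint collecting miscellaneous nodes, apparently as a sample, with no executed logic in its event graph.
; Disconnected nodes cover view target blending, input modes and toggles, teleporting, component attachment, Select and Format Text.
; The one working function, Calculate Money Reward, uses a Math Expression node to multiply scaled player luck by scaled enemy HP.
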(fn ConstructionScript)

(fn CalculateMoneyReward
  (params (PlayerLuck :type Float%20%28double-precision%29) (EnemyHP :type Float%20%28double-precision%29))
  (return (|((PlayerLuck/5)*(EnemyHP/30)) PlayerLuck EnemyHP)))