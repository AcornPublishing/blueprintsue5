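; BP_Tips is an actor holding a few small, independent event snippets, with no single clear game role.
; RoundResult prints a formatted message with the round winner's name and score.
; EquipShield attaches the shield to the skeletal mesh's left arm socket, keeping relative transforms.
; Overlap events enable the actor's player input while a BP_FirstPersonCharacter is inside and disable it on exit.
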(event Custom|Round%20Result
  (params (WinnerName :type String) (WinnerScore :type Integer))
  (Development|PrintText (Utilities|Text|FormatText "{Name} wins the round with {Score}  points" WinnerName WinnerScore)))

(event Custom|Equip%20Shield
  (Transformation|AttachComponentToComponent (Variables|Default|GetShield%20Actor) (Variables|Default|GetSkeletalMesh) "Left ArmSocket" "KeepRelative" "KeepRelative" "KeepRelative" true))

(event EventBeginPlay)

(event Collision|EventActorBeginOverlap
  (params (OtherActor :type Actor%20Object%20Reference))
  (Utilities|Casting|CastToBP_FirstPersonCharacter OtherActor)
  (Input|EnableInput (Game|GetPlayerController 0)))

(event EventTick
  (params (DeltaSeconds :type Float%20%28single-precision%29)))

(event Collision|EventActorEndOverlap
  (params (OtherActor :type Actor%20Object%20Reference))
  (Utilities|Casting|CastToBP_FirstPersonCharacter OtherActor)
  (Input|DisableInput (Game|GetPlayerController 0)))

(fn ConstructionScript)