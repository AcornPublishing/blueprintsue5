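; BP_RandomSpawner spawns an actor of SpawnClass at a random TargetPoints transform on BeginPlay.
; It also holds unrelated flow-control and container samples: Switch, FlipFlop, Sequence, ForEach, set, map and data table lookups.
; Space drives a DoOnce charge weapon with a timed reset and a separate DoN counter that R resets.
; The weapon fire and charge functions are empty stubs.
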(event Custom|Fire%20dual%20wield%20pistol
  (Utilities|FlowControl|FlipFlop
    (:A
      (Utilities|FireLeftPistol))
    (:B
      (Utilities|FireRightPistol))))

(event Custom|End%20of%20Round
  (params (WinnerNames :type String))
  (Utilities|Set|Add (Variables|Default|GetUniqueNames) WinnerNames))

(event Custom|Race%20Result
  (params (Position :type Integer))
  (switch int Position
    (:1
      (Variables|Default|SetMedalName "GOLD"))
    (:2
      (Variables|Default|SetMedalName "SILVER"))
    (:3
      (Variables|Default|SetMedalName "BRONZE"))))

(event Custom|Sequence%20test
  (Utilities|FlowControl|Sequence
    (:then_0
      (Development|PrintString "FIRST")
      (if true
        (Development|PrintString "SECOND")))
    (:then_1
      (Development|PrintString "THIRD"))))

(event Custom|Turn%20on%20all%20lamps
  (for _array_element (Variables|Default|GetRoom%20Lamps)
    (Rendering|SetVisibility (Variables|/Script/Engine.PointLight|GetPointLightComponent _array_element) true false)))

(event Custom|Full%20charge
  (Utilities|FlowControl|DoOnce false) ; enters at Reset
)

(event EventBeginPlay
  (bind _targetpoints (Variables|Default|GetTargetPoints))
  (if (and (Utilities|IsValidClass (Variables|Default|GetSpawnClass)) (Utilities|Array|IsNotEmpty _targetpoints))
    (Game|SpawnActorfromClass (Variables|Default|GetSpawnClass) (Transformation|GetActorTransform (.OutItem (Utilities|Array|Random _targetpoints))) "Undefined" 0 0)))

(event Input|KeyboardEvents|SpaceBar
  (params (Key :type Key%20Structure :default "None"))
  (:Pressed
    (Utilities|FlowControl|DoN 3)))

(event Input|KeyboardEvents|SpaceBar
  (params (Key :type Key%20Structure :default "None"))
  (:Pressed
    (Utilities|FlowControl|DoOnce false
      (:Completed
        (Utilities|UseChargeWeapon
          (:Out
            (Utilities|Time|SetTimerbyEvent (delegate Custom|Full%20charge) 3e+01)))))))

(event Input|KeyboardEvents|R
  (params (Key :type Key%20Structure :default "None"))
  (:Pressed
    (Utilities|FlowControl|DoN 3) ; enters at Reset
  ))

(fn ConstructionScript)

(fn CalculateTotalPrice
  (params (Product%20Name :type String) (Amount :type Float%20%28double-precision%29))
  (return (* Amount (.Value (Utilities|Map|Find (Variables|Default|GetPriceTable) Product%20Name)))))

(fn SelectWeapon
  (params (Weapon%20ID :type Name))
  (bind _returnvalue (Utilities|GetDataTableRow (Variables|Default|GetWeaponTable) Weapon%20ID)
    (:then
      (bind _output_get (Variables|Default|SetCurrentWeapon _returnvalue))
      (Development|PrintString (.Name (Utilities|Struct|BreakWeaponType _output_get))))))